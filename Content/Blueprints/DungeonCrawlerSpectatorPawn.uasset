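; Spectator pawn for a dungeon crawler that lets a player possess the creature or VR pawn they are looking at.
; Pressing F sphere-traces pawns from the camera, then casts the hit to Skeleton, Floating Skull, Mimic, Beholder or FPS Vive pawn classes.
; The controller cached on possession takes over the match, directly with authority or through PossessionRPC when remote.
; The trace leaves debug drawing visible.
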(event `Key|F`
  (params (Key :type "Key Structure" :default "AnyKey"))
  (:`Pressed`
    (`self.TraceAndPosses`)))

(event `TraceAndPosses`
  (bind _myplayercontroller (`self.MyPlayerController`))
  (bind _camera (`self.Camera`))
  (bind _returnvalue (`SceneComponent.K2_GetComponentLocation` _camera))
  (bind _outhit (`KismetSystemLibrary.SphereTraceSingleForObjects` :`Start` _returnvalue :`End` (+ (* (`KismetMathLibrary.GetForwardVector` (`SceneComponent.K2_GetComponentRotation` _camera)) 10000.0) _returnvalue) :`Radius` 35.0 :`ObjectTypes` (`|MakeArray` "ObjectTypeQuery3" :!type "EObjectTypeQuery Enum") :`DrawDebugType` "ForDuration"))
  (bind (_bblockinghit _binitialoverlap _time _location _impactpoint _normal _impactnormal _physmat _hitactor) (`GameplayStatics.BreakHitResult` _outhit))
  (bind _asskeleton_character (cast `/Game/NPCs/Skelington/AI/SkeletonCharacter` _hitactor)
    (:`then`
      (`/Engine/EditorBlueprintResources/ActorMacros.Switch Has Authority`
        (:`Authority`
          (`Controller.Possess` _myplayercontroller _asskeleton_character))
        (:`Remote`
          (`self.PossessionRPC` _myplayercontroller _asskeleton_character))))
    (:`CastFailed`
      (bind _asfloating_skull_character (cast `/Game/NPCs/FloatingSkull/FloatingSkullCharacter` _hitactor)
        (:`then`
          (`/Engine/EditorBlueprintResources/ActorMacros.Switch Has Authority`
            (:`Authority`
              (`Controller.Possess` _myplayercontroller _asfloating_skull_character))
            (:`Remote`
              (`self.PossessionRPC` _myplayercontroller _asfloating_skull_character))))
        (:`CastFailed`
          (bind _asmimic_character (cast `/Game/NPCs/Mimic/MimicCharacter` _hitactor)
            (:`then`
              (`/Engine/EditorBlueprintResources/ActorMacros.Switch Has Authority`
                (:`Authority`
                  (`Controller.Possess` _myplayercontroller _asmimic_character))
                (:`Remote`
                  (`self.PossessionRPC` _myplayercontroller _asmimic_character))))
            (:`CastFailed`
              (bind _asbeholder_character (cast `/Game/NPCs/Beholder/BeholderCharacter` _hitactor)
                (:`then`
                  (`/Engine/EditorBlueprintResources/ActorMacros.Switch Has Authority`
                    (:`Authority`
                      (`Controller.Possess` _myplayercontroller _asbeholder_character))
                    (:`Remote`
                      (`self.PossessionRPC` _myplayercontroller _asbeholder_character))))
                (:`CastFailed`
                  (bind _asfpsvive_pawn_character (cast `/Game/Vive/FPSVive_PawnCharacter` _hitactor))
                  (`/Engine/EditorBlueprintResources/ActorMacros.Switch Has Authority`
                    (:`Authority`
                      (`Controller.Possess` _myplayercontroller _asfpsvive_pawn_character))
                    (:`Remote`
                      (`self.PossessionRPC` _myplayercontroller _asfpsvive_pawn_character))))))))))))

(event `self.ReceivePossessed`
  (params (NewController :type "Controller Object Reference"))
  (`self.StoreplayerController` NewController))

(event `StoreplayerController`
  (params (NewParam :type "Controller Object Reference"))
  (set `self.MyPlayerController` NewParam))

(event `self.ReceiveUnpossessed`
  (params (OldController :type "Controller Object Reference"))
  (set `self.MyPlayerController` null))

(event `PossessionRPC`
  (params (Controller :type "Controller Object Reference") (pawn :type "Pawn Object Reference"))
  (`Controller.Possess` Controller pawn))

(fn `UserConstructionScript`)